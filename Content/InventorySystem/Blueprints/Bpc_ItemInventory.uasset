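; Inventory component that stores items as class and amount pairs in a slot array, sized to AmountOfSlots at BeginPlay.
; Helpers query slots by index and find the first empty slot or non-full stack of a given item.
; AddItem fills a free stack before an empty slot for stackable items, places others one per slot, and recurses for overflow, capping stacks at MaxStackSize.
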(event EventBeginPlay
  (Utilities|Array|Resize (Variables|Default|GetSlots) (Variables|Default|GetAmountOfSlots)))

(fn IsSlotEmpty?
  (params (SlotIndex :type Integer))
  (return (not (Utilities|IsValidClass (.ItemClass (Utilities|Struct|BreaksInventorySlot (Utilities|Array|Get(acopy) (Variables|Default|GetSlots) SlotIndex)))))))

(fn GetItembyIndex
  (params (Index :type Integer))
  (bind _slots (Variables|Default|GetSlots))
  (bind _output (Utilities|Array|Get(acopy) _slots Index))
  (bind (_itemclass _amount) (Utilities|Struct|BreaksInventorySlot _output))
  (if (CallFunction|IsSlotEmpty? Index)
    (return true "" 0)
    (else
      (return false (Utilities|GetClassDefaults _itemclass) _amount))))

(fn SearchEmptySlot
  (bind _array_index (Utilities|Array|ForEachLoopwithBreak (Variables|Default|GetSlots) :!label _label)
    (:LoopBody
      (if (CallFunction|IsSlotEmpty? _array_index)
        (LocalVariables|SetLocalBool (CallFunction|IsSlotEmpty? _array_index))
        (LocalVariables|SetLocalIndex _array_index)
        (goto _label Break)))
    (:Completed
      (return (LocalVariables|GetLocalBool) (LocalVariables|GetLocalIndex)))))

(fn SearchFreeStack
  (params (Item :type Object%20Class%20Reference))
  (bind (_array_element _array_index) (Utilities|Array|ForEachLoopwithBreak (Variables|Default|GetSlots) :!label _label)
    (:LoopBody
      (if (Utilities|IsValidClass (.ItemClass (Utilities|Struct|BreaksInventorySlot _array_element)))
        (if (and (== (.ItemClass (Utilities|Struct|BreaksInventorySlot _array_element)) Item) (< (.Amount (Utilities|Struct|BreaksInventorySlot _array_element)) (Variables|Default|GetMaxStackSize)))
          (LocalVariables|SetLocalBool true)
          (LocalVariables|SetLocalIndex _array_index)
          (goto _label Break))))
    (:Completed
      (return (LocalVariables|GetLocalBool) (LocalVariables|GetLocalIndex)))))

(fn AddItem
  (params (ItemClass :type BP%20Master%20Item%20Class%20Reference) (Amount :type Integer))
  (bind _maxstacksize (Variables|Default|GetMaxStackSize))
  (bind _maxstacksize_2 (Variables|Default|GetMaxStackSize))
  (if (Utilities|Struct|BreaksItemInfo (Utilities|GetClassDefaults ItemClass))
    (bind (_bsuccess_ _index) (CallFunction|SearchFreeStack ItemClass))
    (if _bsuccess_
      (LocalVariables|SetLocalFoundIndex _index)
      (if (> (+ (.Amount (Utilities|Struct|BreaksInventorySlot (Utilities|Array|Get(acopy) (Variables|Default|GetSlots) (LocalVariables|GetLocalFoundIndex)))) Amount) _maxstacksize_2)
        (Utilities|Array|SetArrayElem (Variables|Default|GetSlots) (LocalVariables|GetLocalFoundIndex) (Utilities|Struct|MakesInventorySlot ItemClass _maxstacksize_2))
        (bind _rest (CallFunction|AddItem ItemClass (- Amount (Variables|Default|GetMaxStackSize))))
        (else
          (Utilities|Array|SetArrayElem (Variables|Default|GetSlots) (LocalVariables|GetLocalFoundIndex) (Utilities|Struct|MakesInventorySlot ItemClass (+ (.Amount (Utilities|Struct|BreaksInventorySlot (Utilities|Array|Get(acopy) (Variables|Default|GetSlots) (LocalVariables|GetLocalFoundIndex)))) Amount)))))
      (return true _rest)
      (else
        (bind (_bsuccess__2 _index_2) (CallFunction|SearchEmptySlot))
        (if _bsuccess__2
          (bind _output_get (LocalVariables|SetLocalFoundIndex _index_2))
          (if (> Amount (Variables|Default|GetMaxStackSize))
            (Utilities|Array|SetArrayElem (Variables|Default|GetSlots) _output_get (Utilities|Struct|MakesInventorySlot ItemClass _maxstacksize))
            (bind _rest_2 (CallFunction|AddItem ItemClass (- Amount _maxstacksize)))
            (else
              (Utilities|Array|SetArrayElem (Variables|Default|GetSlots) _output_get (Utilities|Struct|MakesInventorySlot ItemClass Amount))))
          (return true _rest_2)
          (else
            (return false 0)))))
    (else
      (bind (_bsuccess__3 _index_3) (CallFunction|SearchEmptySlot))
      (if _bsuccess__3
        (bind _output_get_2 (LocalVariables|SetLocalFoundIndex _index_3))
        (Utilities|Array|SetArrayElem (Variables|Default|GetSlots) _output_get_2 (Utilities|Struct|MakesInventorySlot ItemClass 1))
        (if (> Amount 1)
          (bind _rest_3 (CallFunction|AddItem ItemClass (- Amount 1))))
        (return true _rest_3)
        (else
          (return false Amount))))))

(fn GetAmountbyIndex
  (params (Index :type Integer))
  (return (.Amount (Utilities|Struct|BreaksInventorySlot (Utilities|Array|Get(acopy) (Variables|Default|GetSlots) Index)))))