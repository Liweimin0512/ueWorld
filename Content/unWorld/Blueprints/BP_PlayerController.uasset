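; BP_PlayerController is a player controller that spawns a BP_SelectedCube at the origin on BeginPlay and keeps a reference to it.
; Its CameraZoom axis adjusts the spring arm length of BP_Player.
; Roll, Attack and the 1 key only cast the pawn to BP_Player.
; Roll, attack, item-add, widget and camera-to-mouse trace logic is present but disconnected, so it never runs.
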(event EventBeginPlay
  (bind _returnvalue (Game|SpawnActorfromClass "/Game/unWorld/Blueprints/Cube/BP_SelectedCube.BP_SelectedCube_C" (Math|Transform|MakeTransform "0, 0, 0") "AlwaysSpawn" 0 0))
  (Variables|Default|SetSelectCube _returnvalue)
  (bind _asbp_player (Utilities|Casting|CastToBP_Player (Game|Player|GetPlayerPawn 0))))

(event EventTick
  (params (DeltaSeconds :type Float%20%28single-precision%29)))

(event Input|ActionEvents|InputActionRoll
  (params (Key :type Key%20Structure :default "None"))
  (:Pressed
    (bind _asbp_player (Utilities|Casting|CastToBP_Player (Game|Player|GetPlayerPawn 0)))))

(event Input|ActionEvents|InputActionChaInfo
  (params (Key :type Key%20Structure :default "None")))

(event Input|ActionEvents|InputActionAttack
  (params (Key :type Key%20Structure :default "None"))
  (:Pressed
    (bind _asbp_player (Utilities|Casting|CastToBP_Player (Game|Player|GetPlayerPawn 0)))))

(event Input|AxisEvents|InputAxisCameraZoom
  (params (AxisValue :type Float%20%28single-precision%29))
  (bind _asbp_player (Utilities|Casting|CastToBP_Player (Game|GetPlayerCharacter 0)))
  (Variables|/Script/Engine.SpringArmComponent|SetTargetArmLength (Variables|/Game/unWorld/Blueprints/BP_Player.BP_Player_C|GetSpringArm _asbp_player) (+ (Variables|/Script/Engine.SpringArmComponent|GetTargetArmLength (Variables|/Game/unWorld/Blueprints/BP_Player.BP_Player_C|GetSpringArm _asbp_player)) (* AxisValue 1e+02))))

(event Input|KeyboardEvents|1
  (params (Key :type Key%20Structure :default "None"))
  (:Pressed
    (bind _asbp_player (Utilities|Casting|CastToBP_Player (Game|Player|GetPlayerPawn 0)))))

(event Input|ActionEvents|InputActionInventory
  (params (Key :type Key%20Structure)))

(fn ConstructionScript)