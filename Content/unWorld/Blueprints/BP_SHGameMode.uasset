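; Game mode that streams an endless grid of BP_Chunk actors around player 0.
; BeginPlay spawns a square of chunks within Radius, and Tick recomputes the player's grid cell from location divided by half of ChunkSize.
; When that cell changes, AddChunk spawns missing chunks at full ChunkSize spacing, tracking actors and integer coordinates in arrays.
; DelChunk is an uncalled stub, so chunks are never removed.
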(event EventBeginPlay
  (CallFunction|GeneratorChunk))

(event EventTick
  (params (DeltaSeconds :type Float%20%28single-precision%29))
  (bind _bupdata_ (CallFunction|UpdatePlayerPosition))
  (if _bupdata_
    (CallFunction|AddChunk)))

(fn ConstructionScript)

(fn GeneratorChunk
  (bind _radius (Variables|Default|GetRadius))
  (bind _radius_2 (Variables|Default|GetRadius))
  (bind _chunksize (Variables|Default|GetChunkSize))
  (for _index (range (* _radius -1) _radius)
    (for _index_2 (range (* _radius_2 -1) _radius_2)
      (bind _returnvalue (Game|SpawnActorfromClass "/Game/unWorld/Blueprints/Cube/BP_Chunk.BP_Chunk_C" (Math|Conversions|ToTransform(Vector) (Math|Vector|MakeVector (* (+ _index (Variables|Default|GetChunkX)) _chunksize) (* (+ _index_2 (Variables|Default|GetChunkY)) _chunksize) 0.0)) "Undefined" 0 0))
      (Utilities|Array|Add (Variables|Default|GetChunk) _returnvalue)
      (Utilities|Array|Add (Variables|Default|GetChunkPosition) (Utilities|Struct|MakeIntVector (+ _index (Variables|Default|GetChunkX)) (+ _index_2 (Variables|Default|GetChunkY)))))))

(fn UpdatePlayerPosition
  (bind _returnvalue (Game|GetPlayerCharacter 0))
  (bind _chunksize (Variables|Default|GetChunkSize))
  (bind _returnvalue_2 (Transformation|GetActorLocation _returnvalue))
  (bind _returnvalue_3 (/ _chunksize 2.0))
  (bind (_x _y) (Math|Vector|BreakVector _returnvalue_2))
  (bind _returnvalue_4 (/ _x _returnvalue_3))
  (bind _returnvalue_5 (/ _y _returnvalue_3))
  (bind _returnvalue_6 (Math|Float|Floor _returnvalue_5))
  (bind _returnvalue_7 (Math|Float|Floor _returnvalue_4))
  (if (and (== (Variables|Default|GetChunkX) _returnvalue_7) (== (Variables|Default|GetChunkY) _returnvalue_6))
    (return false)
    (else
      (Variables|Default|SetChunkX _returnvalue_7)
      (Variables|Default|SetChunkY _returnvalue_6)
      (return true))))

(fn AddChunk
  (bind _radius (Variables|Default|GetRadius))
  (bind _radius_2 (Variables|Default|GetRadius))
  (for _index (range (* _radius_2 -1) _radius_2)
    (for _index_2 (range (* _radius -1) _radius)
      (if (not (Utilities|Array|ContainsItem (Variables|Default|GetChunkPosition) (Utilities|Struct|MakeIntVector (+ _index (Variables|Default|GetChunkX)) (+ _index_2 (Variables|Default|GetChunkY)))))
        (bind _returnvalue (Game|SpawnActorfromClass "/Game/unWorld/Blueprints/Cube/BP_Chunk.BP_Chunk_C" (Math|Conversions|ToTransform(Vector) (Math|Vector|MakeVector (* (+ _index (Variables|Default|GetChunkX)) (Variables|Default|GetChunkSize)) (* (+ _index_2 (Variables|Default|GetChunkY)) (Variables|Default|GetChunkSize)) 0.0)) "Undefined" 0 0))
        (Utilities|Array|Add (Variables|Default|GetChunk) _returnvalue)
        (Utilities|Array|Add (Variables|Default|GetChunkPosition) (Utilities|Struct|MakeIntVector (+ _index (Variables|Default|GetChunkX)) (+ _index_2 (Variables|Default|GetChunkY))))))))

(fn DelChunk
  (for _array_element (Variables|Default|GetChunkPosition)
    _))