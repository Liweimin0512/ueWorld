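; BP_GameMode is a game mode that builds the starting world from chunks and sets up player control when play begins.
; GeneratorChunk uses nested loops to spawn BP_Chunk actors in a flat, evenly spaced square grid from the origin.
; BeginPlay then spawns an actor high above the grid origin for the first player controller to possess, though that spawn node shows no class assigned.
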(event EventBeginPlay
  (CallFunction|GeneratorChunk)
  (bind _returnvalue (Game|SpawnActorfromClass 0 (Math|Transform|MakeTransform "0.000000, 0,5000.000000" "0, 0, 0" "1,1,1") "Undefined" 0 0))
  (Pawn|Possess (Game|GetPlayerController 0) _returnvalue))

(event EventTick
  (params (DeltaSeconds :type Float%20%28single-precision%29)))

(fn ConstructionScript)

(fn GeneratorChunk
  (for _index (range 0 10)
    (for _index_2 (range 0 10)
      (Game|SpawnActorfromClass "/Game/unWorld/Core/Cube/BP_Chunk.BP_Chunk_C" (Math|Conversions|ToTransform(Vector) (Math|Vector|MakeVector (* 1600 (Math|Conversions|ToFloat(Integer) _index)) (* 1600 (Math|Conversions|ToFloat(Integer) _index_2)) 0.0)) "Undefined" 0 0))))