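; Master character Blueprint that provides a health stat bar and ability-driven combat helpers built on the Gameplay Ability System.
; BeginPlay links the W_StatBar widget to its owner, and health changes refresh its text and fill.
; Gameplay tag queries, alive and pause checks gate melee attacks, which activate abilities from the current weapon slot.
; Potion use activates by item slot without those checks; the skill attack is an empty stub.
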(event Custom|DelayedDestroy
  (Actor|DestroyActor))

(event Custom|OnHealthChanged_1
  (params (DeltaValue :type Float%20%28single-precision%29) (EventTags :type Gameplay%20Tag%20Container%20Structure%20%28by%20ref%29))
  (CallFunction|SetStatBar))

(event EventBeginPlay
  (CallFunction|SetStatBar)
  (bind _asw_stat_bar (Utilities|Casting|CastToW_StatBar (UserInterface|GetUserWidgetObject (Variables|Default|GetW_StatBar))))
  (Variables|/Game/unWorld/SkillSystem/Widgets/W_StatBar.W_StatBar_C|SetOwnerCharacter _asw_stat_bar self))

(event Collision|EventActorBeginOverlap
  (params (OtherActor :type Actor%20Object%20Reference)))

(event EventTick
  (params (DeltaSeconds :type Float%20%28single-precision%29)))

(fn ConstructionScript)

(fn SetStatBar
  (bind _returnvalue (Class|UnWorldCharacter|GetHealth))
  (bind _returnvalue_2 (Class|UnWorldCharacter|GetMaxHealth))
  (bind _asw_stat_bar (Utilities|Casting|CastToW_StatBar (UserInterface|GetUserWidgetObject (Variables|Default|GetW_StatBar))))
  (Rendering|Components|TextRender|SetText (Variables|/Game/unWorld/SkillSystem/Widgets/W_StatBar.W_StatBar_C|GetStatText _asw_stat_bar) (Utilities|Text|FormatText "{health}/{maxHealth}" _returnvalue _returnvalue_2))
  (Progress|SetPercent (Variables|/Game/unWorld/SkillSystem/Widgets/W_StatBar.W_StatBar_C|GetStatBar _asw_stat_bar) (/ _returnvalue _returnvalue_2)))

(fn IsAlive
  (return (> (Class|UnWorldCharacter|GetHealth) 0.0)))

(fn IsUsingMelee
  (bind _activeabilities (Class|UnWorldCharacter|GetActiveAbilitieswithTags "(GameplayTags=((TagName=\"Ability.Melee\")))"))
  (return (> (Utilities|Array|Length _activeabilities) 0)))

(fn IsUsingSkill
  (bind _activeabilities (Class|UnWorldCharacter|GetActiveAbilitieswithTags "(GameplayTags=((TagName=\"Ability.Skill\")))"))
  (return (> (Utilities|Array|Length _activeabilities) 0)))

(fn CanUseAnyAbility
  (return (Math|Boolean|ANDBoolean (Health|IsAlive) (not (Game|IsGamePaused)) (not (Animation|IsUsingSkill)))))

(fn DoMeleeAttack
  (if (and (Animation|CanUseAnyAbility) (not (Animation|IsUsingMelee)))
    (bind _returnvalue (Class|UnWorldCharacter|ActivateAbilitieswithItemSlot (Variables|Default|GetCurrentWeaponSlot) true))
    (return _returnvalue)))

(fn DoSkillAttack)

(fn UseItemPotion
  (Class|UnWorldCharacter|ActivateAbilitieswithItemSlot))