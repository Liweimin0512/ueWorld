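; Player controller that handles camera zoom and inventory toggling for BP_PlayerCharacter.
; The CameraZoom axis changes the spring arm length without clamping.
; Inventory input opens or closes W_Inventory, opening only when the character has an InventorySystemComponent.
; Roll, Attack and key 1 only cast the pawn; their actions, plus character-info widget, selection-cube spawn and mouse trace logic, are disconnected.
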(event EventBeginPlay)

(event EventTick
  (params (DeltaSeconds :type Float%20%28single-precision%29)))

(event Input|ActionEvents|InputActionRoll
  (params (Key :type Key%20Structure :default "None"))
  (:Pressed
    (bind _asbp_player_character (Utilities|Casting|CastToBP_PlayerCharacter (Game|Player|GetPlayerPawn 0)))))

(event Input|ActionEvents|InputActionChaInfo
  (params (Key :type Key%20Structure :default "None")))

(event Input|ActionEvents|InputActionAttack
  (params (Key :type Key%20Structure :default "None"))
  (:Pressed
    (bind _asbp_player_character (Utilities|Casting|CastToBP_PlayerCharacter (Game|Player|GetPlayerPawn 0)))))

(event Input|AxisEvents|InputAxisCameraZoom
  (params (AxisValue :type Float%20%28single-precision%29))
  (bind _asbp_player_character (Utilities|Casting|CastToBP_PlayerCharacter (Game|GetPlayerCharacter 0)))
  (Variables|/Script/Engine.SpringArmComponent|SetTargetArmLength (Variables|/Game/unWorld/Core/BP_PlayerCharacter.BP_PlayerCharacter_C|GetSpringArm _asbp_player_character) (+ (Variables|/Script/Engine.SpringArmComponent|GetTargetArmLength (Variables|/Game/unWorld/Core/BP_PlayerCharacter.BP_PlayerCharacter_C|GetSpringArm _asbp_player_character)) (* AxisValue 1e+02))))

(event Input|KeyboardEvents|1
  (params (Key :type Key%20Structure :default "None"))
  (:Pressed
    (bind _asbp_player_character (Utilities|Casting|CastToBP_PlayerCharacter (Game|Player|GetPlayerPawn 0)))))

(event Input|ActionEvents|InputActionInventory
  (params (Key :type Key%20Structure :default "None"))
  (:Pressed
    (Utilities|IsValid (Variables|Default|GetW_Inventory)
      (:Is%20Valid
        (Default|CloseInventory (Variables|Default|GetW_Inventory))
        (Variables|Default|SetW_Inventory 0))
      (:Is%20Not%20Valid
        (Utilities|IsValid (Actor|GetComponentbyClass (Game|GetPlayerCharacter 0) "/Script/unWorld.InventorySystemComponent")
          (:Is%20Valid
            (bind _returnvalue (UserInterface|CreateWidget "/Game/unWorld/InventorySystem/Widgets/W_Inventory.W_Inventory_C" self))
            (bind _output_get (Variables|Default|SetW_Inventory _returnvalue))
            (UserInterface|Viewport|AddtoViewport _output_get 0)))))))

(fn ConstructionScript)